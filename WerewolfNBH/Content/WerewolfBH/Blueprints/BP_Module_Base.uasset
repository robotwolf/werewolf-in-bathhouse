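; BP_Module_Base is a room module actor, apparently a base class, that sizes its bounds box to fit its static mesh.
; The construction script passes both components to Constructor, which stores them, records the mesh's local bounds size as RoomBounds, and sets the box's extent and relative center from those bounds.
; It prints a success message, or a warning if either component is invalid.
; The event graph holds no active logic.
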(fn `Constructor`
  (params (Box :type "BoxComponent Object Reference") (Mesh :type "StaticMeshComponent Object Reference"))
  (locals (`Box Reference` :type "BoxComponent Object Reference") (`Static Mesh Comp` :type "StaticMeshComponent Object Reference"))
  (bind (_min _max) (`StaticMeshComponent.GetLocalBounds` (`local.Static Mesh Comp`)))
  (bind (_min_2 _max_2) (`StaticMeshComponent.GetLocalBounds` (`local.Static Mesh Comp`)))
  (bind _returnvalue (- _max_2 _min_2))
  (if (and (`KismetSystemLibrary.IsValid` Box) (`KismetSystemLibrary.IsValid` Mesh))
    (set `local.Box Reference` Box)
    (set `local.Static Mesh Comp` Mesh)
    (set `self.RoomBounds` _returnvalue)
    (`BoxComponent.SetBoxExtent` (`local.Box Reference`) (/ _returnvalue (2.0 2.0 2.0)) true)
    (`SceneComponent.K2_SetRelativeLocation` (`local.Box Reference`) (/ (+ _min _max) (2.0 2.0 2.0)) false false)
    (`KismetSystemLibrary.PrintString` (`KismetStringLibrary.Concat_StrStr` "BP_Module: " (`KismetSystemLibrary.GetDisplayName` (`self.StaticMesh`)) " completed init SUCCESSFULLY") true true (struct :`G` 0.269565 :`B` 0.014444 :`A` 1.0) 5.0)
    (else
      (`KismetSystemLibrary.PrintString` (`KismetStringLibrary.Concat_StrStr` "BP_Module: " (`KismetSystemLibrary.GetDisplayName` (`self.StaticMesh`)) " has Mesh and/or Box Collision missing.") true true (struct :`R` 1.0 :`G` 0.11377 :`B` 0.000851 :`A` 1.0) 5.0))))

(fn `UserConstructionScript`
  (`self.Constructor` (`self.RoomBoundsBox`) (`self.StaticMesh`)))