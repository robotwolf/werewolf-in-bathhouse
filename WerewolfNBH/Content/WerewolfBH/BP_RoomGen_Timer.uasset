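; BP_RoomGen_Timer is an actor that periodically regenerates room layouts.
; On BeginPlay it loops over all RoomGenerator actors, storing each in a single reference and setting a looping timer on DelayTime.
; Each timer tick calls GenerateLayoutWithNewSeed on that reference, so only the last generator stored is regenerated.
; An invalid reference only prints a debug message.
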(event `self.ReceiveBeginPlay`
  (bind _outactors (`GameplayStatics.GetAllActorsOfClass` "/Script/WerewolfNBH.RoomGenerator"))
  (for _array_element _outactors
    (set `self.Room Generator Ref` _array_element)
    (if (`KismetSystemLibrary.IsValid` (`self.Room Generator Ref`))
      (`KismetSystemLibrary.K2_SetTimer` null "Regenerate" (`self.Delay Time`) true)
      (else
        (`KismetSystemLibrary.PrintString` "Timer: FUCK")))))

(fn `Regenerate`
  (`RoomGenerator.GenerateLayoutWithNewSeed` (`self.Room Generator Ref`)))

(fn `UserConstructionScript`)